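; Sliding double cell door whose Left and Right halves move apart along local Y and back.
; With AUTO set, overlapping the Open component opens it, then it closes after a short pause; otherwise OpenDoor and CloseDoor events drive it.
; Movement uses looping short Delays that step a Progress alpha for vector lerps, in place of a Timeline.
; A DoOnce blocks reopening until closing finishes.
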(event OnComponentBeginOverlap(open)
  (params (OverlappedComponent :type Primitive%20Component%20Object%20Reference) (OtherActor :type Actor%20Object%20Reference) (OtherComp :type Primitive%20Component%20Object%20Reference) (OtherBodyIndex :type Integer) (bFromSweep :type Boolean) (SweepResult :type Hit%20Result%20Structure%20%28by%20ref%29))
  (if (Variables|Default|GetAUTO?)
    (Utilities|FlowControl|DoOnce false :!label _label
      (:Completed
        (Variables|Default|Setprogress (+ 0.025 (Variables|Default|Getprogress)) :!label _label_2)
        (Utilities|FlowControl|Delay 0.001)
        (Transformation|SetRelativeLocation (Variables|Default|Getleft) (Math|Vector|Lerp(Vector) (Variables|Default|GetStartLocationLeft) (Variables|Default|GetEndLocationLeft) (Variables|Default|Getprogress)) false false)
        (Transformation|SetRelativeLocation (Variables|Default|GetRight) (Math|Vector|Lerp(Vector) (Variables|Default|GetStartLocationRight) (Variables|Default|GetEndLocationRight) (Variables|Default|Getprogress)) false false)
        (if (< (Variables|Default|Getprogress) 1.0)
          (goto _label_2)
          (else
            (Utilities|FlowControl|Delay 2.0)
            (Variables|Default|Setprogress 0.0)
            (if (Variables|Default|GetAUTO?)
              (Variables|Default|Setprogress (+ 0.025 (Variables|Default|Getprogress)) :!label _label_3)
              (Utilities|FlowControl|Delay 0.001)
              (Transformation|SetRelativeLocation (Variables|Default|Getleft) (Math|Vector|Lerp(Vector) (Variables|Default|GetEndLocationLeft) (Variables|Default|GetStartLocationLeft) (Variables|Default|Getprogress)) false false)
              (Transformation|SetRelativeLocation (Variables|Default|GetRight) (Math|Vector|Lerp(Vector) (Variables|Default|GetEndLocationRight) (Variables|Default|GetStartLocationRight) (Variables|Default|Getprogress)) false false)
              (if (< (Variables|Default|Getprogress) 1.0)
                (goto _label_3)
                (else
                  (Variables|Default|Setprogress 0.0)
                  (goto _label Reset))))))))))

(event Custom|Open%20Door
  (Utilities|FlowControl|DoOnce false :!label _label
    (:Completed
      (Variables|Default|Setprogress (+ 0.025 (Variables|Default|Getprogress)) :!label _label_2)
      (Utilities|FlowControl|Delay 0.001)
      (Transformation|SetRelativeLocation (Variables|Default|Getleft) (Math|Vector|Lerp(Vector) (Variables|Default|GetStartLocationLeft) (Variables|Default|GetEndLocationLeft) (Variables|Default|Getprogress)) false false)
      (Transformation|SetRelativeLocation (Variables|Default|GetRight) (Math|Vector|Lerp(Vector) (Variables|Default|GetStartLocationRight) (Variables|Default|GetEndLocationRight) (Variables|Default|Getprogress)) false false)
      (if (< (Variables|Default|Getprogress) 1.0)
        (goto _label_2)
        (else
          (Utilities|FlowControl|Delay 2.0)
          (Variables|Default|Setprogress 0.0)
          (if (Variables|Default|GetAUTO?)
            (Variables|Default|Setprogress (+ 0.025 (Variables|Default|Getprogress)) :!label _label_3)
            (Utilities|FlowControl|Delay 0.001)
            (Transformation|SetRelativeLocation (Variables|Default|Getleft) (Math|Vector|Lerp(Vector) (Variables|Default|GetEndLocationLeft) (Variables|Default|GetStartLocationLeft) (Variables|Default|Getprogress)) false false)
            (Transformation|SetRelativeLocation (Variables|Default|GetRight) (Math|Vector|Lerp(Vector) (Variables|Default|GetEndLocationRight) (Variables|Default|GetStartLocationRight) (Variables|Default|Getprogress)) false false)
            (if (< (Variables|Default|Getprogress) 1.0)
              (goto _label_3)
              (else
                (Variables|Default|Setprogress 0.0)
                (goto _label Reset)))))))))

(event Custom|Close%20Door
  (Variables|Default|Setprogress (+ 0.025 (Variables|Default|Getprogress)) :!label _label)
  (Utilities|FlowControl|Delay 0.001)
  (Transformation|SetRelativeLocation (Variables|Default|Getleft) (Math|Vector|Lerp(Vector) (Variables|Default|GetEndLocationLeft) (Variables|Default|GetStartLocationLeft) (Variables|Default|Getprogress)) false false)
  (Transformation|SetRelativeLocation (Variables|Default|GetRight) (Math|Vector|Lerp(Vector) (Variables|Default|GetEndLocationRight) (Variables|Default|GetStartLocationRight) (Variables|Default|Getprogress)) false false)
  (if (< (Variables|Default|Getprogress) 1.0)
    (goto _label)
    (else
      (Variables|Default|Setprogress 0.0)
      (Utilities|FlowControl|DoOnce false) ; enters at Reset
    )))

(event EventBeginPlay
  (bind _output_get (Variables|Default|SetStartLocationRight (Variables|/Script/Engine.SceneComponent|GetRelativeLocation (Variables|Default|GetRight))))
  (Variables|Default|SetEndLocationRight (Math|Vector|MakeVector (.x _output_get) (- (.y _output_get) 1.4e+02) (.z _output_get)))
  (bind _output_get_2 (Variables|Default|SetStartLocationLeft (Variables|/Script/Engine.SceneComponent|GetRelativeLocation (Variables|Default|Getleft))))
  (Variables|Default|SetEndLocationLeft (Math|Vector|MakeVector (.x _output_get_2) (+ 1.4e+02 (.y _output_get_2)) (.z _output_get_2)))
  (Variables|Default|Setprogress 0.0))

(fn ConstructionScript)