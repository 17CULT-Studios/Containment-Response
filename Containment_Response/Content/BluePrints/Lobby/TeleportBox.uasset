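; TeleportBox is a lobby trigger actor that moves an overlapping actor to a Destination location.
; With DebugSpeed on, the move is immediate; otherwise it prints Timer and loops through a one-second Delay while Timer is at least one.
; The loop sets Timer to a negative constant rather than decrementing it, so it waits at most one second.
; Ending overlap sets ErrorCheck to cancel the pending move and resets Timer.
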(event OnActorBeginOverlap(TeleportBox)
  (params (OverlappedActor :type Actor%20Object%20Reference) (OtherActor :type Actor%20Object%20Reference))
  (if (Variables|Default|GetDebug%20Speed)
    (Transformation|SetActorLocation OtherActor (Variables|Default|GetDestination) false false :!label _label)
    (else
      (Variables|Default|SetErrorCheck false)
      (Development|PrintString (Utilities|String|ToString(Float) (Variables|Default|Gettimer)) :!label _label_2)
      (if (not (Variables|Default|GetErrorCheck))
        (if (<= 1.0 (Variables|Default|Gettimer))
          (Variables|Default|Settimer (- 0.0 1.0))
          (Utilities|FlowControl|Delay 1.0)
          (goto _label_2)
          (else
            (goto _label)))))))

(event OnActorEndOverlap(TeleportBox)
  (params (OverlappedActor :type Actor%20Object%20Reference) (OtherActor :type Actor%20Object%20Reference))
  (Variables|Default|SetErrorCheck true)
  (Variables|Default|Settimer 1e+01))

(fn ConstructionScript)